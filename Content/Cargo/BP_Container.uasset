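; Cargo container that a BP_Hook can sling and release with four cables.
; Its box trigger toggles a guide hook and registers or clears the container as the hook's capture candidate.
; Slinging briefly moves the hook to the center point, binds cables and four physics constraints to its connector, then restores the hook's position.
; Constraint limits derive from sling-point spacing; Unsling hides the cables and breaks the constraints.
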(event OnComponentBeginOverlap(boxTrigger)
  (params (OverlappedComponent :type Primitive%20Component%20Object%20Reference) (OtherActor :type Actor%20Object%20Reference) (OtherComp :type Primitive%20Component%20Object%20Reference) (OtherBodyIndex :type Integer) (bFromSweep :type Boolean) (SweepResult :type Hit%20Result%20Structure%20%28by%20ref%29))
  (bind _asbp_hook (Utilities|Casting|CastToBP_Hook OtherActor))
  (if (and (Utilities|ClassIsChildOf (Utilities|GetClass OtherActor) "/Game/WorkingCrane/BP_Hook.BP_Hook_C") (not (Variables|/Game/WorkingCrane/BP_Hook.BP_Hook_C|Getcaptured _asbp_hook)))
    (CallFunction|TriggerGuideHook false)
    (bind _asbp_hook_2 (Utilities|Casting|CastToBP_Hook OtherActor))
    (Variables|/Game/WorkingCrane/BP_Hook.BP_Hook_C|SetmayCaptureObject _asbp_hook_2 true)
    (Variables|/Game/WorkingCrane/BP_Hook.BP_Hook_C|SetcapturingObject _asbp_hook_2 self)))

(event OnComponentEndOverlap(boxTrigger)
  (params (OverlappedComponent :type Primitive%20Component%20Object%20Reference) (OtherActor :type Actor%20Object%20Reference) (OtherComp :type Primitive%20Component%20Object%20Reference) (OtherBodyIndex :type Integer))
  (bind _asbp_hook (Utilities|Casting|CastToBP_Hook OtherActor))
  (if (or (and (Utilities|ClassIsChildOf (Utilities|GetClass OtherActor) "/Game/WorkingCrane/BP_Hook.BP_Hook_C") (not (Variables|/Game/WorkingCrane/BP_Hook.BP_Hook_C|Getcaptured _asbp_hook))) (Variables|/Game/WorkingCrane/BP_Hook.BP_Hook_C|Getcaptured _asbp_hook))
    (CallFunction|TriggerGuideHook true)
    (bind _asbp_hook_2 (Utilities|Casting|CastToBP_Hook OtherActor))
    (Variables|/Game/WorkingCrane/BP_Hook.BP_Hook_C|SetmayCaptureObject _asbp_hook_2 false)
    (Variables|/Game/WorkingCrane/BP_Hook.BP_Hook_C|SetcapturingObject _asbp_hook_2 0)))

(fn ConstructionScript)

(fn TriggerGuideHook
  (params (hidden :type Boolean))
  (Development|SetHiddeninGame (Variables|Default|GetguideHook) hidden false))

(fn Slinging
  (params (captrureDevice :type BP%20Hook%20Object%20Reference))
  (bind _connector (Variables|/Game/WorkingCrane/BP_Hook.BP_Hook_C|Getconnector captrureDevice))
  (bind _cable1 (Variables|Default|GetCable1))
  (bind _container (Variables|Default|GetContainer))
  (bind _hook (Variables|/Game/WorkingCrane/BP_Hook.BP_Hook_C|Gethook captrureDevice))
  (bind _output_get (Variables|/Game/WorkingCrane/BP_Hook.BP_Hook_C|SetoldLocation captrureDevice (Transformation|GetWorldLocation _hook)))
  (Variables|/Game/WorkingCrane/BP_Hook.BP_Hook_C|SetlastCapturedObject captrureDevice self)
  (Transformation|SetWorldLocation _hook (+ (Transformation|GetWorldLocation (Variables|Default|GetcenterPoint)) "") false false)
  (CallFunction|SetCablesandConstraintLenght (|((c*(sqrt(2)))/2) (Math|Float|Absolute(Float) (|(x1-x2) (.y (Variables|/Script/Engine.SceneComponent|GetRelativeLocation (Variables|Default|GetslingPoint2))) (.y (Variables|/Script/Engine.SceneComponent|GetRelativeLocation (Variables|Default|GetslingPoint4)))))))
  (Class|CableComponent|SetAttachEndtoComponent _cable1 _connector "None")
  (Variables|/Script/CableComponent.CableComponent|SetEndLocation _cable1 "0, 0, 0")
  (Variables|/Script/CableComponent.CableComponent|SetEndLocation (Variables|Default|GetCable2) "0, 0, 0")
  (Variables|/Script/CableComponent.CableComponent|SetEndLocation (Variables|Default|GetCable3) "0, 0, 0")
  (Variables|/Script/CableComponent.CableComponent|SetEndLocation (Variables|Default|GetCable4) "0, 0, 0")
  (Rendering|SetVisibility (Variables|Default|GetCable1) true false)
  (Physics|SetSimulatePhysics _container false)
  (Utilities|FlowControl|Sequence
    (:then_0
      (Class|PhysicsConstraintComponent|SetConstrainedComponents (Variables|Default|GetPhysicsConstraint1) _connector "None" (Variables|Default|GetslingPoint1) "None"))
    (:then_1
      (Class|PhysicsConstraintComponent|SetConstrainedComponents (Variables|Default|GetPhysicsConstraint2) _connector "None" (Variables|Default|GetslingPoint2) "None"))
    (:then_2
      (Class|PhysicsConstraintComponent|SetConstrainedComponents (Variables|Default|GetPhysicsConstraint3) _connector "None" (Variables|Default|GetslingPoint3) "None"))
    (:then_3
      (Class|PhysicsConstraintComponent|SetConstrainedComponents (Variables|Default|GetPhysicsConstraint4) _connector "None" (Variables|Default|GetslingPoint4) "None"))
    (:then_4
      (Physics|SetSimulatePhysics _container true)
      (Variables|/Game/WorkingCrane/BP_Hook.BP_Hook_C|Setcaptured captrureDevice true)
      (Transformation|SetWorldLocation _hook _output_get false false))))

(fn CalculateHeightOfHook
  (params (X1 :type Float%20%28double-precision%29) (X2 :type Float%20%28double-precision%29))
  (return (|(x/2) (Math|Float|Absolute(Float) (|(x1-x2) X1 X2)))))

(fn MoveHooktoPoint
  (params (objectToMove :type BP%20Hook%20Object%20Reference) (endPoint :type Vector)))

(fn SetCablesandConstraintLenght
  (params (lenght :type Float%20%28double-precision%29))
  (Variables|/Script/CableComponent.CableComponent|SetCableLength (Variables|Default|GetCable1) 1e+02)
  (Variables|/Script/CableComponent.CableComponent|SetCableLength (Variables|Default|GetCable2) 1e+02)
  (Variables|/Script/CableComponent.CableComponent|SetCableLength (Variables|Default|GetCable3) 1e+02)
  (Variables|/Script/CableComponent.CableComponent|SetCableLength (Variables|Default|GetCable4) 1e+02)
  (Class|PhysicsConstraintComponent|SetLinearZLimit (Variables|Default|GetPhysicsConstraint1) "LCM_Limited" (+ lenght 1e+02)))

(fn Unsling
  (params (capturingDevice :type BP%20Hook%20Object%20Reference))
  (bind _cable1 (Variables|Default|GetCable1))
  (bind _container (Variables|Default|GetContainer))
  (Class|CableComponent|SetAttachEndtoComponent _cable1 0 "None")
  (Rendering|SetVisibility _cable1 false false)
  (Physics|SetSimulatePhysics _container true)
  (Class|PhysicsConstraintComponent|BreakConstraint (Variables|Default|GetPhysicsConstraint1))
  (Physics|SetSimulatePhysics _container true)
  (Variables|/Game/WorkingCrane/BP_Hook.BP_Hook_C|Setcaptured capturingDevice false)
  (Variables|/Game/WorkingCrane/BP_Hook.BP_Hook_C|SetlastCapturedObject capturingDevice 0))

(fn CalculateHookLocation
  (params (Capturing%20device :type BP%20Hook%20Object%20Reference))
  (bind _height (CallFunction|CalculateHeightOfHook (.y (Variables|/Script/Engine.SceneComponent|GetRelativeLocation (Variables|Default|GetslingPoint2))) (.y (Variables|/Script/Engine.SceneComponent|GetRelativeLocation (Variables|Default|GetslingPoint4)))))
  (return (+ (Transformation|GetWorldLocation (Variables|Default|GetcenterPoint)) (Math|Vector|MakeVector 0.0 0.0 _height))))