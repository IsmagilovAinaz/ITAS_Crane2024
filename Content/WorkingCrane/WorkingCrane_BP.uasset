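; Player-controlled working crane with rail travel, tower rotation, boom reach and hoisting, plus cargo capture.
; Input shifts gears on four BPEngine components and updates the HUD; AsyncPhysicsTick applies their velocities to the actor, ABP_WorkingCrane and cables.
; The BP_Hook hangs on four cable components paired with physics constraints, whose Z limits change with cable length.
; Capture moves the hook over cargo by Timeline, then slings directly or through Slinger_AI.
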(event `SlingingEvent`
  (bind _capturedevice (`self.captureDevice`))
  ;[1 1 1] Захват Объекта (Кнопка E)
  (`/Game/Cargo/BP_Container.Slinging` (stale `InputAction|CaptureObject` _output_get) _capturedevice :!label _label)
  (`PrimitiveComponent.SetSimulatePhysics` (`/Game/WorkingCrane/BP_Hook.hook` _capturedevice) true))

(event `InputAction|CaptureObject`
  (params (Key :type "Key Structure"))
  (bind _capturedevice (`self.captureDevice`))
  (bind _capturingobject (`/Game/WorkingCrane/BP_Hook.capturingObject` _capturedevice))
  (bind _hook (`/Game/WorkingCrane/BP_Hook.hook` _capturedevice))
  (bind _lastcapturedobject (`/Game/WorkingCrane/BP_Hook.lastCapturedObject` _capturedevice))
  (bind _captured (`/Game/WorkingCrane/BP_Hook.captured` _capturedevice))
  (bind (_returnvalue_x _returnvalue_y _returnvalue_z) (`KismetMathLibrary.BreakVector` (`SceneComponent.K2_GetComponentLocation` _hook)))
  ;[1 1 1] Захват Объекта (Кнопка E)
  (:`Pressed`
    (if (and (and (`/Game/WorkingCrane/BP_Hook.mayCaptureObject` _capturedevice) (`KismetSystemLibrary.IsValid` _capturingobject)) (not _captured))
      (bind _output_get (set `/Game/WorkingCrane/BP_Hook.lastCapturedObject` _capturingobject _capturedevice))
      (`PrimitiveComponent.SetSimulatePhysics` (`/Game/WorkingCrane/BP_Hook.hook` _capturedevice) false)
      (bind _newpos (`/Game/Cargo/BP_Container.Calculate Hook Location` _capturingobject _capturedevice))
      (bind (_direction _newtrack_2) (`Timeline|Timeline`)
        (:`Update`
          (bind (_returnvalue_x_2 _returnvalue_y_2 _returnvalue_z_2) (`KismetMathLibrary.BreakVector` (`KismetMathLibrary.VLerp` (`KismetMathLibrary.MakeVector` _returnvalue_x _returnvalue_y _returnvalue_z) (`KismetMathLibrary.MakeVector` (.x _newpos) (.y _newpos) (- (.z _newpos) 400.0)) _newtrack_2)))
          (if (< _returnvalue_z _returnvalue_z_2)
            _
            (else
              _))
          (`SceneComponent.K2_SetWorldLocation` _hook (`KismetMathLibrary.MakeVector` _returnvalue_x_2 _returnvalue_y_2 _returnvalue_z_2) false false))
        (:`Finished`
          (if (`self.slingerFlag`)
            (if (`self.NotFirstSling`)
              (`self.Slinger Unpause `)
              (else
                (bind _returnvalue (`GameplayStatics.GetActorOfClass` "/Game/Slinger/AI_Logic/Slinger_AI.Slinger_AI_C"))
                (bind _asslinger_ai (cast `/Game/Slinger/AI_Logic/Slinger_AI` _returnvalue))
                (`/Game/Slinger/AI_Logic/Slinger_AI.startSlinging` _asslinger_ai)))
            (else
              (goto _label)))))
      (elif (and _captured (`KismetSystemLibrary.IsValid` _lastcapturedobject))
        (if (`self.slingerFlag`)
          (`self.Slinger Unpause `)
          (else
            (`/Game/Cargo/BP_Container.Unsling` _lastcapturedobject _capturedevice :!label _label_2)))))))

(event `InputAction|ReachForward`
  (params (Key :type "Key Structure"))
  (bind _bp_enginereach (`self.BP_EngineReach`))
  (bind _gears (`/Game/WorkingCrane/BP_Engine.gears` (`self.BP_EngineReach`)))
  ;[1 1 1] Повышение/понижение передачи вылета стрелы (R - вперед, F - назад)
  (:`Pressed`
    (if (< _gears 2)
      (bind _result (`/Engine/EditorBlueprintResources/StandardMacros.IncrementInt` _gears)
        (:`  `
          (`KismetSystemLibrary.PrintText` (`KismetTextLibrary.Conv_IntToText` _result))
          (if true :!label _label_3
            (`/Game/WorkingCrane/BP_Engine.GearChanging` _bp_enginereach)
            (`self.updateHUD` 2 (`KismetTextLibrary.Conv_DoubleToText` (`KismetMathLibrary.Conv_IntToDouble` (`/Game/WorkingCrane/BP_Engine.gears` _bp_enginereach)) "HalfToEven"))))))))

(event `InputAction|LiftCables`
  (params (Key :type "Key Structure"))
  (bind _bp_enginecables (`self.BP_EngineCables`))
  (bind _gears (`/Game/WorkingCrane/BP_Engine.gears` (`self.BP_EngineCables`)))
  ;[1 1 1] Повышение/понижение передачи изменения длины тросса (Z - Разматывание, X - Сматиывание)
  (:`Pressed`
    (if (< _gears 3)
      (bind _result (`/Engine/EditorBlueprintResources/StandardMacros.IncrementInt` _gears)
        (:`  `
          (if true :!label _label_4
            (`/Game/WorkingCrane/BP_Engine.GearChanging` _bp_enginecables)
            (`self.updateHUD` 3 (`KismetTextLibrary.Conv_IntToText` (`/Game/WorkingCrane/BP_Engine.gears` _bp_enginecables)))))))))

(event `InputAction|ReachBackward`
  (params (Key :type "Key Structure"))
  (bind _gears (`/Game/WorkingCrane/BP_Engine.gears` (`self.BP_EngineReach`)))
  ;[1 1 1] Повышение/понижение передачи вылета стрелы (R - вперед, F - назад)
  (:`Pressed`
    (if (> _gears -2)
      (bind _result (`/Engine/EditorBlueprintResources/StandardMacros.DecrementInt` _gears)
        (:`  `
          (`KismetSystemLibrary.PrintText` (`KismetTextLibrary.Conv_IntToText` _result))
          (goto _label_3))))))

(event `Unsling Event`
  ;[1 1 1] Захват Объекта (Кнопка E)
  (set `self.NotFirstSling` true)
  (goto _label_2))

(event `InputAction|LowerCables`
  (params (Key :type "Key Structure"))
  (bind _gears (`/Game/WorkingCrane/BP_Engine.gears` (`self.BP_EngineCables`)))
  ;[1 1 1] Повышение/понижение передачи изменения длины тросса (Z - Разматывание, X - Сматиывание)
  (:`Pressed`
    (if (> _gears -3)
      (bind _result (`/Engine/EditorBlueprintResources/StandardMacros.DecrementInt` _gears)
        (:`  `
          (goto _label_4))))))

(event `InputAction|UpshiftRails`
  (params (Key :type "Key Structure"))
  (bind _bp_enginemove (`self.BP_EngineMove`))
  (bind _gears (`/Game/WorkingCrane/BP_Engine.gears` (`self.BP_EngineMove`)))
  ;[1 1 1] Повышение/понижение передачи движения крана (W - вперед / S - назад)
  (:`Pressed`
    (if (< _gears 2)
      (bind _result (`/Engine/EditorBlueprintResources/StandardMacros.IncrementInt` _gears)
        (:`  `
          (if true :!label _label_5
            (`/Game/WorkingCrane/BP_Engine.GearChanging` _bp_enginemove)
            (`self.updateHUD` 0 (`KismetTextLibrary.Conv_IntToText` (`/Game/WorkingCrane/BP_Engine.gears` _bp_enginemove)))))))))

(event `InputAction|RotateTowerRight`
  (params (Key :type "Key Structure"))
  (bind _bp_enginerotate (`self.BP_EngineRotate`))
  (bind _gears (`/Game/WorkingCrane/BP_Engine.gears` (`self.BP_EngineRotate`)))
  ;[1 1 1] Повышение/понижение передачи поворота башни (A - влево, D - право, left arrow, right arrow)
  (:`Pressed`
    (if (< _gears 2)
      (bind _result (`/Engine/EditorBlueprintResources/StandardMacros.IncrementInt` _gears)
        (:`  `
          (if true :!label _label_6
            (`/Game/WorkingCrane/BP_Engine.GearChanging` _bp_enginerotate)
            (`self.updateHUD` 1 (`KismetTextLibrary.Conv_IntToText` (`/Game/WorkingCrane/BP_Engine.gears` _bp_enginerotate)))))))))

(event `InputAction|DownshiftRails`
  (params (Key :type "Key Structure"))
  (bind _gears (`/Game/WorkingCrane/BP_Engine.gears` (`self.BP_EngineMove`)))
  ;[1 1 1] Повышение/понижение передачи движения крана (W - вперед / S - назад)
  (:`Pressed`
    (if (> _gears -2)
      (bind _result (`/Engine/EditorBlueprintResources/StandardMacros.DecrementInt` _gears)
        (:`  `
          (goto _label_5))))))

(event `InputAction|RotateTowerLeft`
  (params (Key :type "Key Structure"))
  (bind _gears (`/Game/WorkingCrane/BP_Engine.gears` (`self.BP_EngineRotate`)))
  ;[1 1 1] Повышение/понижение передачи поворота башни (A - влево, D - право, left arrow, right arrow)
  (:`Pressed`
    (if (> _gears -2)
      (bind _result (`/Engine/EditorBlueprintResources/StandardMacros.DecrementInt` _gears)
        (:`  `
          (goto _label_6))))))

(event `InputAxis|MouseUpDown`
  (params (AxisValue :type "Float (single-precision)"))
  ;[1 1 1] Вращение головой
  (`self.AddControllerPitchInput` AxisValue))

(event `self.ReceiveAsyncPhysicsTick`
  (params (DeltaSeconds :type "Float (single-precision)") (SimSeconds :type "Float (single-precision)"))
  (bind _bp_enginecables (`self.BP_EngineCables`))
  (bind _sphere (`self.Sphere`))
  (bind (_returnvalue_roll _returnvalue_pitch _returnvalue_yaw) (`KismetMathLibrary.BreakRotator` (`SceneComponent.K2_GetComponentRotation` _sphere)))
  (bind _gears (`/Game/WorkingCrane/BP_Engine.gears` _bp_enginecables))
  (bind (_returnvalue_x _returnvalue_y _returnvalue_z) (`KismetMathLibrary.BreakVector` (`SceneComponent.K2_GetComponentLocation` (`/Game/WorkingCrane/BP_Hook.connector` (`self.captureDevice`)))))
  ;[1 1 1] Перемещение крана
  (`|ExecutionSequence`
    (:`then_0`
      (bind _outputvel (`/Game/WorkingCrane/BP_Engine.CalculateOutputVelocity` (`self.BP_EngineMove`) SimSeconds))
      (`self.K2_AddActorWorldOffset` (* (`self.GetActorForwardVector`) _outputvel)))
    (:`then_1`
      ;[1 1 1] Поворот башни крана
      (bind _outputvel_2 (`/Game/WorkingCrane/BP_Engine.CalculateOutputVelocity` (`self.BP_EngineRotate`) SimSeconds))
      (bind _asabp_working_crane (cast `/Game/WorkingCrane/ABP_WorkingCrane` (`SkeletalMeshComponent.GetAnimInstance` (`self.SkeletalMesh`))))
      (bind (_rotatetower_roll _rotatetower_pitch _rotatetower_yaw) (`KismetMathLibrary.BreakRotator` (`/Game/WorkingCrane/ABP_WorkingCrane.rotateTower` _asabp_working_crane)))
      (set `/Game/WorkingCrane/ABP_WorkingCrane.rotateTower` (`KismetMathLibrary.MakeRotator` 0.0 0.0 (+ _outputvel_2 _rotatetower_yaw)) _asabp_working_crane))
    (:`then_2`
      ;[1 1 1] Изменение длины троссов
      (bind _outputvel_3 (`/Game/WorkingCrane/BP_Engine.CalculateOutputVelocity` _bp_enginecables SimSeconds))
      (bind _returnvalue (`PhysicsConstraintComponent.GetConstraint` (`self.PhysicsConstraint`)))
      (bind (_xmotion _ymotion _zmotion _limit) (`ConstraintInstanceBlueprintLibrary.GetLinearLimits` _returnvalue))
      (if (not (or (and (<= (- _returnvalue_z 15.0) 0.0) (> _gears 0)) (and (<= _limit (`self.minLenght`)) (< _gears 0))))
        (bind _returnvalue_2 (/ _outputvel_3 1.0))
        (`PhysicsConstraintComponent.SetLinearZLimit` (`self.PhysicsConstraint`) "LCM_Limited" (+ _returnvalue_2 _limit))
        (`PhysicsConstraintComponent.SetLinearZLimit` (`self.PhysicsConstraint1`) "LCM_Limited" (+ _returnvalue_2 _limit))
        (`PhysicsConstraintComponent.SetLinearZLimit` (`self.PhysicsConstraint2`) "LCM_Limited" (+ _returnvalue_2 _limit))
        (`PhysicsConstraintComponent.SetLinearZLimit` (`self.PhysicsConstraint3`) "LCM_Limited" (+ _returnvalue_2 _limit))
        (`self.addCablesLenght` _returnvalue_2)))
    (:`then_3`
      ;[1 1 1] Вылет стрелы
      (bind _outputvel_4 (`/Game/WorkingCrane/BP_Engine.CalculateOutputVelocity` (`self.BP_EngineReach`) SimSeconds))
      (bind _asabp_working_crane_2 (cast `/Game/WorkingCrane/ABP_WorkingCrane` (`SkeletalMeshComponent.GetAnimInstance` (`self.SkeletalMesh`))))
      (set `/Game/WorkingCrane/ABP_WorkingCrane.reachSpeed` (+ (`/Game/WorkingCrane/ABP_WorkingCrane.reachSpeed` _asabp_working_crane_2) _outputvel_4) _asabp_working_crane_2)
      ;[1 1 1] При вылете стрелы изменяется вращение сокета по X сбрасываем значение чтобы constraint смотрел строго вниз
      (`SceneComponent.K2_SetWorldRotation` _sphere (`KismetMathLibrary.MakeRotator` 0.0 _returnvalue_pitch _returnvalue_yaw) false false)
      (`SceneComponent.K2_SetWorldRotation` (`self.Sphere1`) (`KismetMathLibrary.MakeRotator` 0.0 _returnvalue_pitch _returnvalue_yaw) false false)
      (`SceneComponent.K2_SetWorldRotation` (`self.Sphere2`) (`KismetMathLibrary.MakeRotator` 0.0 _returnvalue_pitch _returnvalue_yaw) false false)
      (`SceneComponent.K2_SetWorldRotation` (`self.Sphere3`) (`KismetMathLibrary.MakeRotator` 0.0 _returnvalue_pitch _returnvalue_yaw) false false))))

(event `self.ReceiveBeginPlay`
  (bind _sphere (`self.Sphere`))
  (bind _cable (`self.Cable`))
  (bind _cable3 (`self.Cable3`))
  (bind _cable2 (`self.Cable2`))
  (bind _cable1 (`self.Cable1`))
  (bind _cableslenght (`self.cablesLenght`))
  (bind (_returnvalue_roll _returnvalue_pitch _returnvalue_yaw) (`KismetMathLibrary.BreakRotator` (`SceneComponent.K2_GetComponentRotation` _sphere)))
  ;[1 1 1] Привязка троссов к крюку при прогрузке уровня
  (bind _returnvalue (`GameplayStatics.GetActorOfClass` "/Game/WorkingCrane/BP_Hook.BP_Hook_C"))
  (bind _output_get (set `self.captureDevice` _returnvalue))
  (`SceneComponent.K2_SetWorldRotation` _sphere (`KismetMathLibrary.MakeRotator` 0.0 _returnvalue_pitch _returnvalue_yaw) false false)
  (`SceneComponent.K2_SetWorldRotation` (`self.Sphere1`) (`KismetMathLibrary.MakeRotator` 0.0 _returnvalue_pitch _returnvalue_yaw) false false)
  (`SceneComponent.K2_SetWorldRotation` (`self.Sphere2`) (`KismetMathLibrary.MakeRotator` 0.0 _returnvalue_pitch _returnvalue_yaw) false false)
  (`SceneComponent.K2_SetWorldRotation` (`self.Sphere3`) (`KismetMathLibrary.MakeRotator` 0.0 _returnvalue_pitch _returnvalue_yaw) false false)
  (`PrimitiveComponent.SetSimulatePhysics` (`/Game/WorkingCrane/BP_Hook.hook` _output_get) false)
  (bind _defaultsceneroot (`/Game/WorkingCrane/BP_Hook.DefaultSceneRoot` _output_get))
  (`SceneComponent.K2_SetWorldLocation` _defaultsceneroot (+ (`SceneComponent.K2_GetComponentLocation` (`self.pointOfJoint`)) (`KismetMathLibrary.MakeVector` 0.0 0.0 (* -1.0 _cableslenght))) false false)
  (`SceneComponent.K2_SetWorldLocation` (`/Game/WorkingCrane/BP_Hook.hook` _output_get) (+ (`SceneComponent.K2_GetComponentLocation` (`self.pointOfJoint`)) (`KismetMathLibrary.MakeVector` 0.0 0.0 (* -1.0 _cableslenght))) false false)
  (`SceneComponent.K2_SetWorldRotation` _defaultsceneroot (`SceneComponent.K2_GetComponentRotation` (`self.DefaultSceneRoot`)) false false)
  (`self.setCablesLenght` _cableslenght)
  (`PhysicsConstraintComponent.SetLinearZLimit` (`self.PhysicsConstraint3`) "LCM_Limited" _cableslenght)
  (`PhysicsConstraintComponent.SetLinearZLimit` (`self.PhysicsConstraint2`) "LCM_Limited" _cableslenght)
  (`PhysicsConstraintComponent.SetLinearZLimit` (`self.PhysicsConstraint1`) "LCM_Limited" _cableslenght)
  (`PhysicsConstraintComponent.SetLinearZLimit` (`self.PhysicsConstraint`) "LCM_Limited" _cableslenght)
  (bind _sphere_2 (`/Game/WorkingCrane/BP_Hook.Sphere` _output_get))
  (`CableComponent.SetAttachEndToComponent` _cable _sphere_2 "None")
  (bind _sphere1 (`/Game/WorkingCrane/BP_Hook.Sphere1` _output_get))
  (`CableComponent.SetAttachEndToComponent` _cable1 _sphere1 "None")
  (bind _sphere3 (`/Game/WorkingCrane/BP_Hook.Sphere3` _output_get))
  (`CableComponent.SetAttachEndToComponent` _cable2 _sphere3 "None")
  (bind _sphere2 (`/Game/WorkingCrane/BP_Hook.Sphere2` _output_get))
  (`CableComponent.SetAttachEndToComponent` _cable3 _sphere2 "None")
  (`PhysicsConstraintComponent.SetConstrainedComponents` (`self.PhysicsConstraint`) (`self.Sphere`) "None" _sphere_2 "None")
  (`PhysicsConstraintComponent.SetConstrainedComponents` (`self.PhysicsConstraint1`) (`self.Sphere1`) "None" _sphere1 "None")
  (`PhysicsConstraintComponent.SetConstrainedComponents` (`self.PhysicsConstraint2`) (`self.Sphere2`) "None" _sphere3 "None")
  (`PhysicsConstraintComponent.SetConstrainedComponents` (`self.PhysicsConstraint3`) (`self.Sphere3`) "None" _sphere2 "None")
  (set `CableComponent.EndLocation` (0.0 0.0 0.0) _cable)
  (set `CableComponent.EndLocation` (0.0 0.0 0.0) _cable3)
  (set `CableComponent.EndLocation` (0.0 0.0 0.0) _cable2)
  (set `CableComponent.EndLocation` (0.0 0.0 0.0) _cable1)
  (`PrimitiveComponent.SetSimulatePhysics` (`/Game/WorkingCrane/BP_Hook.hook` (`self.captureDevice`)) true))

(event `InputAxis|MouseRightLeft`
  (params (AxisValue :type "Float (single-precision)"))
  ;[1 1 1] Вращение головой
  (`self.AddControllerYawInput` AxisValue))

(fn `addCablesLenght`
  (params (newLenght :type "Float (double-precision)"))
  (bind _cable (`self.Cable`))
  (bind _returnvalue (+ newLenght (`CableComponent.CableLength` _cable)))
  (set `CableComponent.CableLength` _returnvalue _cable)
  (set `CableComponent.CableLength` _returnvalue (`self.Cable1`))
  (set `CableComponent.CableLength` _returnvalue (`self.Cable2`))
  (set `CableComponent.CableLength` _returnvalue (`self.Cable3`))
  (set `self.cablesLenght` _returnvalue))

(fn `CalculateVelocity`
  (params (k :type "Float (double-precision)") (colVelocity :type "Float (double-precision)") (t1 :type "Float (double-precision)") (t2 :type "Float (double-precision)") (elapsTime :type "Float (double-precision)"))
  (returns (outVel :type "Float (double-precision)"))
  (return (+ colVelocity (* k (+ (- 1.0 (* (/ t1 (- t1 t2)) (`KismetMathLibrary.Exp` (/ (* -1.0 elapsTime) t1)))) (* (/ t2 (- t1 t2)) (`KismetMathLibrary.Exp` (/ (* -1.0 elapsTime) t2))))))))

(fn `CalculateVelocity_0`
  (params (deltaTime :type "Float (double-precision)"))
  (returns (outVel :type "Float (double-precision)"))
  (set `self.timeElapsed` (+ (`self.timeElapsed`) deltaTime))
  (bind _output_get (set `self.outputVelocityRails` (+ (`self.colectedVelocityRails`) (* (`self.k`) (+ (- 1.0 (* (/ (`self.t1`) (- (`self.t1`) (`self.t2`))) (`KismetMathLibrary.Exp` (/ (* -1.0 (`self.timeElapsed`)) (`self.t1`))))) (* (/ (`self.t2`) (- (`self.t1`) (`self.t2`))) (`KismetMathLibrary.Exp` (/ (* -1.0 (`self.timeElapsed`)) (`self.t2`)))))))))
  (return _output_get))

(fn `movePhysicsConstraintToMidleOfRopes`
  (params (HooksWorldLoc :type "Vector Structure") (Z :type "Float (double-precision)"))
  (bind _physicsconstraint2 (`self.PhysicsConstraint2`))
  (bind _physicsconstraint3 (`self.PhysicsConstraint3`))
  (bind _physicsconstraint1 (`self.PhysicsConstraint1`))
  (bind _physicsconstraint (`self.PhysicsConstraint`))
  (bind _physicsconstraint_2 (`self.PhysicsConstraint`))
  (bind (_returnvalue_x _returnvalue_y) (`KismetMathLibrary.BreakVector` (`SceneComponent.K2_GetComponentLocation` _physicsconstraint3)))
  (bind (_returnvalue_x_2 _returnvalue_y_2 _returnvalue_z) (`KismetMathLibrary.BreakVector` (`SceneComponent.K2_GetComponentLocation` (`self.PhysicsConstraint`))))
  (bind (_returnvalue_x_3 _returnvalue_y_3) (`KismetMathLibrary.BreakVector` (`SceneComponent.K2_GetComponentLocation` _physicsconstraint1)))
  (bind (_returnvalue_x_4 _returnvalue_y_4) (`KismetMathLibrary.BreakVector` (`SceneComponent.K2_GetComponentLocation` _physicsconstraint2)))
  (bind (_returnvalue_x_5 _returnvalue_y_5) (`KismetMathLibrary.BreakVector` (`SceneComponent.K2_GetComponentLocation` _physicsconstraint)))
  (bind _returnvalue (- _returnvalue_z Z))
  (`SceneComponent.K2_SetWorldLocation` _physicsconstraint (`KismetMathLibrary.MakeVector` _returnvalue_x_5 _returnvalue_y_5 _returnvalue) false false)
  (`SceneComponent.K2_SetWorldLocation` _physicsconstraint1 (`KismetMathLibrary.MakeVector` _returnvalue_x_3 _returnvalue_y_3 _returnvalue) false false)
  (`SceneComponent.K2_SetWorldLocation` _physicsconstraint2 (`KismetMathLibrary.MakeVector` _returnvalue_x_4 _returnvalue_y_4 _returnvalue) false false)
  (`SceneComponent.K2_SetWorldLocation` _physicsconstraint3 (`KismetMathLibrary.MakeVector` _returnvalue_x _returnvalue_y _returnvalue) false false)
  (`SceneComponent.K2_SetRelativeLocation` _physicsconstraint_2 (* (`SceneComponent.RelativeLocation` _physicsconstraint_2) 2.0) false false))

(fn `ReleaseCargo`
  (params (captureDevice :type "/Game/WorkingCrane/BP_Hook Object Reference")))

(fn `setCablesLenght`
  (params (newLenght :type "Float (double-precision)"))
  (set `CableComponent.CableLength` newLenght (`self.Cable`))
  (set `CableComponent.CableLength` newLenght (`self.Cable1`))
  (set `CableComponent.CableLength` newLenght (`self.Cable2`))
  (set `CableComponent.CableLength` newLenght (`self.Cable3`))
  (set `self.cablesLenght` newLenght))

(fn `SetTime`
  (params (T1 :type "Float (double-precision)") (T2 :type "Float (double-precision)"))
  (set `self.t1` T1)
  (set `self.t2` T2))

(fn `updateHUD`
  (params (EngineType :type Integer) (text :type Text))
  (bind _asnew_hud (cast `/Game/WorkingCrane/NewHUD` (`PlayerController.GetHUD` (`GameplayStatics.GetPlayerController` 0))))
  (`/Game/WorkingCrane/NewWidgetBlueprint.Update Text` (`/Game/WorkingCrane/NewHUD.UI_ref` _asnew_hud) EngineType text))

(fn `UserConstructionScript`)